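; Combat manager Blueprint that starts combat on BeginPlay and runs one round of sequential turns.
; It gathers BP_CombatantBase components from "Combatant"-tagged actors into a TurnOrder map keyed to Initiative, passes it through ProcessCombatants and prints the returned values.
; Each combatant's turn-ended event advances the index and triggers the next TakeTurn, clearing InCombat after the last.
; Registration, removal, win checks, EndTurn and IsCombatActive are empty stubs.
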(event `self.ReceiveBeginPlay`
  (`self.StartCombat`))

(event `CombatStarted`
  (bind _keypin (`|MapForEach` (`self.TurnOrder`))
    (:`then`
      (add `/Game/Blueprints/Combatant/BP_CombatantBase.CombatantTurnEnded` _keypin (delegate `TurnEnded`)))))

(event `TurnEnded`
  (bind _currentturnindex (`self.CurrentTurnIndex`))
  (`KismetSystemLibrary.PrintString` "Ended a turn" true true (struct :`R` 1.0 :`A` 1.0))
  (set `self.CurrentTurnIndex` (+ _currentturnindex 1))
  (if (< _currentturnindex (`BlueprintMapLibrary.Map_Length` (`self.TurnOrder`)))
    (`self.StartTurn`)
    (else
      (`KismetSystemLibrary.PrintString` "All turns done" true true (struct :`R` 1.0 :`B` 0.773914 :`A` 1.0))
      (set `self.InCombat` false))))

(fn `CheckWinConditions`)

(fn `EndTurn`)

(fn `GetAllCombatants`
  (bind _outactors (`GameplayStatics.GetAllActorsWithTag` "Combatant"))
  (for _array_element _outactors
    (bind _returnvalue (`self.GetComponentByClass` _array_element "/Game/Blueprints/Combatant/BP_CombatantBase.BP_CombatantBase_C"))
    (if (`KismetSystemLibrary.IsValid` _returnvalue)
      (`KismetArrayLibrary.Array_Add` (`self.CombatantList`) _returnvalue)))
  (for _array_element_2 (`self.CombatantList`)
    (`BlueprintMapLibrary.Map_Add` (`self.TurnOrder`) _array_element_2 (`/Game/Blueprints/Combatant/BP_CombatantBase.Initiative` _array_element_2)))
  (bind _returnvalue_2 (`self.ProcessCombatants` (`self.TurnOrder`)))
  (bind _values (`BlueprintMapLibrary.Map_Values` _returnvalue_2))
  (for _array_element_3 _values
    (`KismetSystemLibrary.PrintString` (`KismetStringLibrary.Conv_DoubleToString` _array_element_3))))

(fn `IsCombatActive`)

(fn `RegisterCombatant`)

(fn `RemoveCombatant`)

(fn `StartCombat`
  (set `self.InCombat` true)
  (`self.GetAllCombatants`)
  (`self.CombatStarted`)
  (`self.StartTurn`)
  (`KismetSystemLibrary.PrintString` "Combat done"))

(fn `StartTurn`
  (if (`self.InCombat`)
    (`/Game/Blueprints/Combatant/BP_CombatantBase.TakeTurn` (`BlueprintMapLibrary.Map_GetKeyValueByIndex` (`self.TurnOrder`) (`self.CurrentTurnIndex`)))))

(fn `UserConstructionScript`)